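; Cone_01 is an actor that gets sucked into the player on contact, in the manner of a collectible.
; When the player pawn overlaps its Trigger, a timeline pulls it toward the pawn's live location, shrinks it to zero scale and switches off its PointLight.
; Each update lerps from the current transform rather than a stored start, and the actor destroys itself when the timeline finishes.
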(event OnComponentBeginOverlap(Trigger)
  (params (OverlappedComponent :type Primitive%20Component%20Object%20Reference) (OtherActor :type Actor%20Object%20Reference) (OtherComp :type Primitive%20Component%20Object%20Reference) (OtherBodyIndex :type Integer) (bFromSweep :type Boolean) (SweepResult :type Hit%20Result%20Structure%20%28by%20ref%29))
  (if (== OtherActor (Game|Player|GetPlayerPawn 0))
    (bind (_direction _01 _02) (Timeline|Timeline_0 Play)
      (:Update
        (Transformation|SetActorLocation (Math|Vector|Lerp(Vector) (Transformation|GetActorLocation) (Transformation|GetActorLocation (Game|Player|GetPlayerPawn 0)) _01) false false)
        (Transformation|SetActorScale3D (Math|Vector|Lerp(Vector) (Transformation|GetActorScale3D) "0, 0, 0" _02))
        (Rendering|Components|Light|SetIntensity (Variables|Default|GetPointLight) 0.0))
      (:Finished
        (Actor|DestroyActor)))))

(fn ConstructionScript)